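; BP_Shop is a shop Blueprint that opens and closes the item-buying widget.
; OpenWidget creates a WB_BuyItem widget, adds it to the viewport, shows the mouse cursor and switches player 0 to Game and UI input focused on it.
; CloseWidget removes the stored widget if it is valid, clears the reference, restores game-only input and hides the cursor.
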(event `Open Widget`
  (bind _returnvalue (`GameplayStatics.GetPlayerController` 0))
  (bind _returnvalue_2 (`|CreateWidget` "/Game/Blueprints/Shop/WB_BuyItem.WB_BuyItem_C"))
  (bind _output_get (set `self.Buy Item Widget` _returnvalue_2))
  (`UserWidget.AddToViewport` _output_get 0)
  (set `PlayerController.bShowMouseCursor` true _returnvalue)
  (`WidgetBlueprintLibrary.SetInputMode_GameAndUIEx` _returnvalue (`self.Buy Item Widget`)))

(event `Close Widget`
  (bind _returnvalue (`GameplayStatics.GetPlayerController` 0))
  (bind _buy_item_widget (`self.Buy Item Widget`)
    (:`then`
      (`Widget.RemoveFromParent` _buy_item_widget)
      (set `self.Buy Item Widget` null)
      (`WidgetBlueprintLibrary.SetInputMode_GameOnly` _returnvalue)
      (set `PlayerController.bShowMouseCursor` false _returnvalue))
    (:`else`)))

(fn `UserConstructionScript`)