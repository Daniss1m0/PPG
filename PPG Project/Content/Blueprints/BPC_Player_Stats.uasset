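; Player stats component that tracks current and max health and stamina for BP_PlayerCharacter.
; On BeginPlay it waits one tick, caches the owning character and initializes the HUD bars and health text.
; Each increase, decrease or max-change function writes the new value straight to the character's HUD widget.
; Increases clamp to the max, while decreases return true once the stat is at or below zero, without clamping.
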(event `self.ReceiveBeginPlay`
  (bind _hud_widget (`/Game/Blueprints/BP_PlayerCharacter.HUD Widget` (`self.Player Character BP`)))
  (`KismetSystemLibrary.DelayUntilNextTick`)
  (bind _asbp_player_character (cast `/Game/Blueprints/BP_PlayerCharacter` (`self.GetOwner`)))
  (set `self.Player Character BP` _asbp_player_character)
  (`ProgressBar.SetPercent` (`/Game/UI/WB_HUD.StaminaBar` (`/Game/Blueprints/BP_PlayerCharacter.HUD Widget` (`self.Player Character BP`))) (/ (`self.Current Stamina`) (`self.Max Stamina`)))
  (`ProgressBar.SetPercent` (`/Game/UI/WB_HUD.HealthBar` _hud_widget) (/ (`self.Current Health`) (`self.Max Health`)))
  (`TextBlock.SetText` (`/Game/UI/WB_HUD.HealthText` _hud_widget) (`KismetTextLibrary.Conv_DoubleToText` (`self.Current Health`) "HalfToEven")))

(fn `Decrease Health`
  (params (Damage :type "Float (double-precision)"))
  (returns (`Is Player Dead?` :type Boolean))
  (bind _hud_widget (`/Game/Blueprints/BP_PlayerCharacter.HUD Widget` (`self.Player Character BP`)))
  (if (not (<= (`self.Current Health`) 0.0))
    (bind _output_get (set `self.Current Health` (- (`self.Current Health`) Damage)))
    (`ProgressBar.SetPercent` (`/Game/UI/WB_HUD.HealthBar` _hud_widget) (/ _output_get (`self.Max Health`)))
    (`TextBlock.SetText` (`/Game/UI/WB_HUD.HealthText` _hud_widget) (`KismetTextLibrary.Conv_DoubleToText` (`self.Current Health`) "HalfToEven"))
    (if (<= (`self.Current Health`) 0.0)
      _
      (else
        (return false))))
  (return true))

(fn `Decrease Stamina`
  (params (`Stamina Depleted` :type "Float (double-precision)"))
  (returns (`Not Stamin Left` :type Boolean))
  (if (not (<= (`self.Current Stamina`) 0.0))
    (set `self.Current Stamina` (- (`self.Current Stamina`) `Stamina Depleted`))
    (`ProgressBar.SetPercent` (`/Game/UI/WB_HUD.StaminaBar` (`/Game/Blueprints/BP_PlayerCharacter.HUD Widget` (`self.Player Character BP`))) (/ (`self.Current Stamina`) (`self.Max Stamina`)))
    (if (<= (`self.Current Stamina`) 0.0)
      _
      (else
        (return false))))
  (return true))

(fn `Increase Health`
  (params (`Added Health` :type "Float (double-precision)"))
  (bind _hud_widget (`/Game/Blueprints/BP_PlayerCharacter.HUD Widget` (`self.Player Character BP`)))
  (set `self.Current Health` (+ (`self.Current Health`) `Added Health`))
  (if (> (`self.Current Health`) (`self.Max Health`))
    (set `self.Current Health` (`self.Max Health`)))
  (`ProgressBar.SetPercent` (`/Game/UI/WB_HUD.HealthBar` _hud_widget) (/ (`self.Current Health`) (`self.Max Health`)))
  (`TextBlock.SetText` (`/Game/UI/WB_HUD.HealthText` _hud_widget) (`KismetTextLibrary.Conv_DoubleToText` (`self.Current Health`) "HalfToEven")))

(fn `Increase Max Health`
  (params (`Health Incremention` :type "Float (double-precision)"))
  (bind _hud_widget (`/Game/Blueprints/BP_PlayerCharacter.HUD Widget` (`self.Player Character BP`)))
  (set `self.Max Health` (+ (`self.Max Health`) `Health Incremention`))
  (`ProgressBar.SetPercent` (`/Game/UI/WB_HUD.HealthBar` _hud_widget) (/ (`self.Current Health`) (`self.Max Health`)))
  (`TextBlock.SetText` (`/Game/UI/WB_HUD.HealthText` _hud_widget) (`KismetTextLibrary.Conv_DoubleToText` (`self.Current Health`) "HalfToEven")))

(fn `Increase Max Stamina`
  (params (`Added Stamina` :type "Float (double-precision)"))
  (set `self.Max Stamina` (+ (`self.Max Stamina`) `Added Stamina`))
  (`ProgressBar.SetPercent` (`/Game/UI/WB_HUD.StaminaBar` (`/Game/Blueprints/BP_PlayerCharacter.HUD Widget` (`self.Player Character BP`))) (/ (`self.Current Stamina`) (`self.Max Stamina`))))

(fn `Increase Stamina`
  (params (`Added Stamina` :type "Float (double-precision)"))
  (set `self.Current Stamina` (+ (`self.Current Stamina`) `Added Stamina`))
  (if (> (`self.Current Stamina`) (`self.Max Stamina`))
    (set `self.Current Stamina` (`self.Max Stamina`)))
  (`ProgressBar.SetPercent` (`/Game/UI/WB_HUD.StaminaBar` (`/Game/Blueprints/BP_PlayerCharacter.HUD Widget` (`self.Player Character BP`))) (/ (`self.Current Stamina`) (`self.Max Stamina`))))