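; BP_NPC is a non-player character with dialogue, a floating name tag and a health bar.
; On BeginPlay it passes its dialogue data to the dialog component, links itself to the name widget and caches the health bar UI.
; Each Tick turns the health bar toward the player camera.
; Projectile hits on the capsule reduce health through the stats component; a true result ragdolls the mesh and hides both widgets.
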(event `self.ReceiveTick`
  (params (DeltaSeconds :type "Float (single-precision)"))
  (`SceneComponent.K2_SetWorldRotation` (`self.Health Bar Widget`) (`KismetMathLibrary.FindLookAtRotation` (`SceneComponent.K2_GetComponentLocation` (`self.Health Bar Widget`)) (`SceneComponent.K2_GetComponentLocation` (`PlayerCameraManager.TransformComponent` (`GameplayStatics.GetPlayerCameraManager` 0)))) false false))

(event `self.CapsuleComponent.OnComponentHit`
  (params (HitComponent :type "PrimitiveComponent Object Reference") (OtherActor :type "Actor Object Reference") (OtherComp :type "PrimitiveComponent Object Reference") (NormalImpulse :type "Vector Structure") (Hit :type "HitResult Structure (by ref)"))
  (cast `/Game/Blueprints/BP_Projectile` OtherActor)
  (bind _is_player_dead_ (`/Game/Blueprints/BPC_Player_Stats.Decrease Health` (`self.BPC_Player_Stats`) 10.0))
  (if _is_player_dead_
    (`PrimitiveComponent.SetSimulatePhysics` (`self.Mesh`) true)
    (`SceneComponent.SetVisibility` (`self.Health Bar Widget`) false false)
    (`SceneComponent.SetVisibility` (`self.Name Widget`) false false)))

(event `self.ReceiveBeginPlay`
  (set `/Game/Blueprints/NPC/Dialog_System/BP_DialogComponent.DialogDatabase` (`self.DialogData`) (`self.BP_DialogComponent`))
  (bind _aswb_npcname (cast `/Game/UI/WB_NPCName` (`WidgetComponent.GetWidget` (`self.Name Widget`))))
  (set `/Game/UI/WB_NPCName.Owner BluePrint` self _aswb_npcname)
  (bind _aswb_npchelth_bar (cast `/Game/UI/WB_NPCHealthBar` (`WidgetComponent.GetWidget` (`self.Health Bar Widget`))))
  (set `self.Health Bar UI` _aswb_npchelth_bar))

(fn `UserConstructionScript`)