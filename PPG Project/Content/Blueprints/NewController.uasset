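; NewController is a controller Blueprint that manages the set of currently selected units, apparently for RTS-style unit selection.
; Three functions add a unit without duplicates, remove one, or clear the whole UnitSelection array, calling IsSelected on each affected unit to keep its selected state in sync.
; The event graph and construction script are empty, so nothing in this Blueprint calls these functions.
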(fn `AddUnitToSelection`
  (params (UnitBase :type "/Game/Blueprints/NPC/BP_NPC_Enemy Object Reference"))
  (`KismetArrayLibrary.Array_AddUnique` (`self.UnitSelection`) UnitBase)
  (`/Game/Blueprints/NPC/BP_NPC_Enemy.IsSelected` UnitBase true))

(fn `ClearUnitSelection`
  (for _array_element (`self.UnitSelection`)
    (`/Game/Blueprints/NPC/BP_NPC_Enemy.IsSelected` _array_element false))
  (`KismetArrayLibrary.Array_Clear` (`self.UnitSelection`)))

(fn `RemoveUnitFromSelection`
  (params (Unit :type "/Game/Blueprints/NPC/BP_NPC_Enemy Object Reference"))
  (`KismetArrayLibrary.Array_RemoveItem` (`self.UnitSelection`) Unit)
  (`/Game/Blueprints/NPC/BP_NPC_Enemy.IsSelected` Unit false))

(fn `UserConstructionScript`)