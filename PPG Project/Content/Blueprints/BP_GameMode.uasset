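; Game mode that scatters weapon pickups across random spawn points when play begins.
; SpawnPages gathers every BP_SpawnPoint, then in a short fixed-count loop spawns a BP_Weapon at a randomly chosen point's location.
; Each used point is removed from the local list and destroyed, so no location repeats.
; Despite the function's name, the spawned actors are weapons.
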(event `self.ReceiveBeginPlay`
  (`self.SpawnPages`))

(fn `SpawnPages`
  (locals (localSpawnPoins :type "Array of /Game/Blueprints/BP_SpawnPoint Object Reference") (localItem :type "/Game/Blueprints/BP_SpawnPoint Object Reference"))
  (bind _outactors (`GameplayStatics.GetAllActorsOfClass` "/Game/Blueprints/BP_SpawnPoint.BP_SpawnPoint_C"))
  (set `local.localSpawnPoins` _outactors)
  (for _ (range 3)
    (set `local.localItem` (`KismetArrayLibrary.Array_Random` (`local.localSpawnPoins`)))
    (`|SpawnActorFromClass` "/Game/Equipment_System/BP_Weapon.BP_Weapon_C" (`KismetMathLibrary.MakeTransform` (`self.K2_GetActorLocation` (`local.localItem`))) "AdjustIfPossibleButAlwaysSpawn" "MultiplyWithRoot" null (struct) null)
    (`KismetArrayLibrary.Array_RemoveItem` (`local.localSpawnPoins`) (`local.localItem`))
    (`self.K2_DestroyActor` (`local.localItem`))))

(fn `UserConstructionScript`)