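; Equipment component for the player character that picks up weapons and keeps their item data in a weapon slot list.
; On BeginPlay it caches the owning BP_PlayerCharacter's camera.
; Pressing E sphere-traces forward from that camera against WorldDynamic objects, with debug drawing, then stores a hit BP_Weapon's ItemData and destroys the actor.
; A debug key on H prints each stored item's row name.
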(event EventBeginPlay
  (bind _asbp_player_character (Utilities|Casting|CastToBP_PlayerCharacter (Components|GetOwner)))
  (Variables|Default|SetCamera%200 (Variables|/Game/Blueprints/BP_PlayerCharacter.BP_PlayerCharacter_C|GetCamera0 _asbp_player_character)))

(event Input|KeyboardEvents|DebugKeyH
  (params (Key :type Key%20Structure :default "None") (ActionValue :type Input%20Action%20Value%20Structure))
  ;[1 1 1] Pick Up Trace
  (:Pressed
    (for _array_element (Variables|Default|GetweaponSlots)
      (Development|PrintString (Utilities|String|ToString(Name) (.rowname (.item _array_element))) true true "(R=0.000000,G=0.660000,B=1.000000,A=1.000000)" 5.0))))

(event Input|KeyboardEvents|E
  (params (Key :type Key%20Structure :default "None"))
  (bind _camera_0 (Variables|Default|GetCamera%200))
  (bind _returnvalue (Transformation|GetWorldLocation _camera_0))
  ;[1 1 1] Pick Up Trace
  (:Pressed
    (bind (_outhit _returnvalue_2) (Collision|SphereTraceForObjects _returnvalue (+ _returnvalue (* (Math|Vector|GetForwardVector (Transformation|GetWorldRotation _camera_0)) 1e+03)) 15.0 (Utilities|Array|MakeArray "ObjectTypeQuery2") false 0 "ForDuration"))
    (if _returnvalue_2
      (bind _asbp_weapon (Utilities|Casting|CastToBP_Weapon (.HitActor (Collision|BreakHitResult _outhit))))
      (CallFunction|AddWeapon (Variables|/Game/Equipment_System/BP_Weapon.BP_Weapon_C|GetitemData _asbp_weapon))
      (Actor|DestroyActor _asbp_weapon)
      (Development|PrintString "Item Gathered!"))))

(fn AddWeapon
  (params (NewItem :type S%20Slots%20Structure%20%28by%20ref%29))
  (Utilities|Array|Add (Variables|Default|GetweaponSlots) NewItem))